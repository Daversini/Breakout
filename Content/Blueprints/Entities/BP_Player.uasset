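; BP_Player is the paddle of a brick-breaker style game, following the mouse cursor along the X axis.
; Each tick it sets the Player component to the cursor trace's X, keeping its Y and a fixed height.
; It spawns a BP_Ball at BallSpawn shortly after play begins and plays a hit sound when the ball overlaps PlayerColl.
; A ball overlapping DeathColl reloads the current level after a short delay.
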(event OnComponentBeginOverlap(PlayerColl)
  (params (OverlappedComponent :type Primitive%20Component%20Object%20Reference) (OtherActor :type Actor%20Object%20Reference) (OtherComp :type Primitive%20Component%20Object%20Reference) (OtherBodyIndex :type Integer) (bFromSweep :type Boolean) (SweepResult :type Hit%20Result%20Structure%20%28by%20ref%29))
  (bind _asbp_ball (Utilities|Casting|CastToBP_Ball OtherActor))
  (Utilities|IsValid _asbp_ball
    (:Is%20Valid
      (Audio|PlaySound2D "/Game/Sounds/BrickHit.BrickHit" 1.0 0.8 0.5 0 0))))

(event OnComponentBeginOverlap(DeathColl)
  (params (OverlappedComponent :type Primitive%20Component%20Object%20Reference) (OtherActor :type Actor%20Object%20Reference) (OtherComp :type Primitive%20Component%20Object%20Reference) (OtherBodyIndex :type Integer) (bFromSweep :type Boolean) (SweepResult :type Hit%20Result%20Structure%20%28by%20ref%29))
  (bind _asbp_ball (Utilities|Casting|CastToBP_Ball OtherActor))
  (Utilities|IsValid _asbp_ball
    (:Is%20Valid
      (Utilities|FlowControl|Delay 1.0)
      (bind _returnvalue (Game|GetCurrentLevelName true))
      (Game|OpenLevel(byName) (Utilities|String|StringToName _returnvalue)))))

(event EventBeginPlay
  (Utilities|FlowControl|Delay 0.5)
  (Game|SpawnActorfromClass "/Game/Blueprints/Entities/BP_Ball.BP_Ball_C" (Transformation|GetWorldTransform (Variables|Default|GetBallSpawn)) "Undefined" 0 0))

(event EventTick
  (params (DeltaSeconds :type Float%20%28single-precision%29))
  (bind _player (Variables|Default|GetPlayer))
  (Transformation|SetWorldLocation _player (Math|Vector|MakeVector (.X (Math|Vector|BreakVector (.location (.HitResult (Game|Player|GetHitResultUnderCursorbyChannel (Game|GetPlayerController 0) "TraceTypeQuery1" true))))) (.y (Transformation|GetWorldLocation _player)) 1e+02) false false))

(fn ConstructionScript)